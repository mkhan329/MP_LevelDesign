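; BP_Mortar is a mortar actor that periodically lobs BP_Bullet projectiles and is destroyed when a BP_Player hits its capsule.
; A loop started on BeginPlay spawns a bullet above the actor, then repeats after a random delay of a few seconds.
; Each bullet's projectile movement gets a fixed horizontal speed along the Arrow's forward vector plus a random upward velocity, varying the arc.
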(event `self.ReceiveBeginPlay`
  (bind (_returnvalue_x _returnvalue_y) (`KismetMathLibrary.BreakVector` (`SceneComponent.GetForwardVector` (`self.Arrow1`))))
  (bind _returnvalue (`|SpawnActorFromClass` "/Game/BluePrints/BP_Bullet.BP_Bullet_C" (`KismetMathLibrary.MakeTransform` (+ (`self.K2_GetActorLocation`) (0.0 0.0 120.0))) "AlwaysSpawn" "MultiplyWithRoot" null null :!label _label))
  (`ProjectileMovementComponent.SetVelocityInLocalSpace` (`/Game/BluePrints/BP_Bullet.ProjectileMovement` _returnvalue) (`KismetMathLibrary.MakeVector` (* _returnvalue_x 750.0) (* _returnvalue_y 750.0) (`KismetMathLibrary.RandomFloatInRange` 500.0 1500.0)))
  (`KismetSystemLibrary.Delay` (`KismetMathLibrary.RandomFloatInRange` 5.0 7.0))
  (goto _label))

(event `self.ReceiveTick`
  (params (DeltaSeconds :type "Float (single-precision)")))

(event `self.CapsuleComponent.OnComponentHit`
  (params (HitComponent :type "PrimitiveComponent Object Reference") (OtherActor :type "Actor Object Reference") (OtherComp :type "PrimitiveComponent Object Reference") (NormalImpulse :type "Vector Structure") (Hit :type "HitResult Structure (by ref)"))
  (cast `/Game/BluePrints/BP_Player` OtherActor)
  (`self.K2_DestroyActor`))

(fn `UserConstructionScript`)