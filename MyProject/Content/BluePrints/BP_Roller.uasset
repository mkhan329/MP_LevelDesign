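; BP_Roller is a moving hazard that damages and knocks back BP_Player.
; Tick slides it along its local X axis by a fixed step per frame, without sweep or delta-time scaling.
; A Cylinder hit applies damage and launches the player away horizontally with added upward lift.
; A player overlapping its Box component destroys the roller.
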(event `self.ReceiveTick`
  (params (DeltaSeconds :type "Float (single-precision)"))
  (`self.K2_AddActorLocalOffset` (* (`KismetMathLibrary.GetForwardVector` (struct)) 4.0)))

(event `self.Box.OnComponentBeginOverlap`
  (params (OverlappedComponent :type "PrimitiveComponent Object Reference") (OtherActor :type "Actor Object Reference") (OtherComp :type "PrimitiveComponent Object Reference") (OtherBodyIndex :type Integer) (bFromSweep :type Boolean) (SweepResult :type "HitResult Structure (by ref)"))
  (cast `/Game/BluePrints/BP_Player` OtherActor)
  (`self.K2_DestroyActor`))

(event `self.Cylinder.OnComponentHit`
  (params (HitComponent :type "PrimitiveComponent Object Reference") (OtherActor :type "Actor Object Reference") (OtherComp :type "PrimitiveComponent Object Reference") (NormalImpulse :type "Vector Structure") (Hit :type "HitResult Structure (by ref)"))
  (bind _asbp_player (cast `/Game/BluePrints/BP_Player` OtherActor))
  (`GameplayStatics.ApplyDamage` _asbp_player 10.0)
  (bind (_returnvalue_x _returnvalue_y) (`KismetMathLibrary.BreakVector` (`KismetMathLibrary.GetDirectionUnitVector` (`self.K2_GetActorLocation`) (`self.K2_GetActorLocation` _asbp_player))))
  (bind (_returnvalue_x_2 _returnvalue_y_2) (`KismetMathLibrary.BreakVector` (`KismetMathLibrary.Normal` (`KismetMathLibrary.MakeVector` _returnvalue_x _returnvalue_y))))
  (`self.LaunchCharacter` _asbp_player (* (`KismetMathLibrary.MakeVector` _returnvalue_x_2 _returnvalue_y_2 1.0) 750.0) false false))

(fn `UserConstructionScript`)