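; BP_Bullet is a projectile that acts as a proximity blast against the player when it bounces.
; On bounce, a player within a fixed radius takes damage and is launched away along the flattened direction from the bullet, with added upward lift.
; The bullet destroys itself after the bounce check whether or not the player is in range, or on Tick once its sphere falls below a height threshold.
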(event `self.ReceiveBeginPlay`)

(event `self.ReceiveTick`
  (params (DeltaSeconds :type "Float (single-precision)"))
  (bind (_returnvalue_x _returnvalue_y _returnvalue_z) (`KismetMathLibrary.BreakVector` (`SceneComponent.K2_GetComponentLocation` (`self.Sphere`))))
  (if (< _returnvalue_z -200.0)
    (`self.K2_DestroyActor`)))

(event `self.ProjectileMovement.OnProjectileBounce`
  (params (ImpactResult :type "HitResult Structure (by ref)") (ImpactVelocity :type "Vector Structure (by ref)"))
  (bind _returnvalue (`GameplayStatics.GetPlayerCharacter` 0))
  (if (<= (`KismetMathLibrary.Vector_Distance` (`self.K2_GetActorLocation` _returnvalue) (`self.K2_GetActorLocation`)) 1000.0)
    (bind _asbp_player (cast `/Game/BluePrints/BP_Player` _returnvalue))
    (`GameplayStatics.ApplyDamage` _asbp_player 10.0)
    (bind (_returnvalue_x _returnvalue_y) (`KismetMathLibrary.BreakVector` (`KismetMathLibrary.GetDirectionUnitVector` (`self.K2_GetActorLocation`) (`self.K2_GetActorLocation` _asbp_player))))
    (bind (_returnvalue_x_2 _returnvalue_y_2) (`KismetMathLibrary.BreakVector` (`KismetMathLibrary.Normal` (`KismetMathLibrary.MakeVector` _returnvalue_x _returnvalue_y))))
    (`Character.LaunchCharacter` _asbp_player (* (`KismetMathLibrary.MakeVector` _returnvalue_x_2 _returnvalue_y_2 1.0) 750.0) false false))
  (`self.K2_DestroyActor`))

(fn `UserConstructionScript`)