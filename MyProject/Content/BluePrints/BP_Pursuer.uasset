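; BP_Pursuer is an enemy pawn that roams, chases the player on sight, and damages and launches them away and upward on hit.
; An AIState switch picks random roaming or chasing via AI MoveTo, re-evaluated one second after each move request.
; Pawn sensing sets the chase state, and a retriggerable delay reverts it to roam shortly after sightings stop.
; The player overlapping its Sphere component destroys the pursuer.
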(event `self.ReceiveHit`
  (params (MyComp :type "PrimitiveComponent Object Reference") (Other :type "Actor Object Reference") (OtherComp :type "PrimitiveComponent Object Reference") (bSelfMoved :type Boolean) (HitLocation :type "Vector Structure") (HitNormal :type "Vector Structure") (NormalImpulse :type "Vector Structure") (Hit :type "HitResult Structure (by ref)"))
  (bind _asbp_player (cast `/Game/BluePrints/BP_Player` Other))
  (`GameplayStatics.ApplyDamage` _asbp_player 10.0)
  (bind (_returnvalue_x _returnvalue_y) (`KismetMathLibrary.BreakVector` (`KismetMathLibrary.GetDirectionUnitVector` (`self.K2_GetActorLocation`) (`self.K2_GetActorLocation` _asbp_player))))
  (bind (_returnvalue_x_2 _returnvalue_y_2) (`KismetMathLibrary.BreakVector` (`KismetMathLibrary.Normal` (`KismetMathLibrary.MakeVector` _returnvalue_x _returnvalue_y))))
  (`self.LaunchCharacter` _asbp_player (* (`KismetMathLibrary.MakeVector` _returnvalue_x_2 _returnvalue_y_2 1.0) 750.0) false false))

(event `Chase Player`
  (`|AIMoveTo` self (0.0 0.0 0.0) (`GameplayStatics.GetPlayerCharacter` 0)
    (:`then`
      (`KismetSystemLibrary.Delay` 1.0)
      (switch `/Game/BluePrints/EAIState` (`self.AIState`) :!label _label
        (:`NewEnumerator1`
          (`self.MoveToRandomLocation`))
        (:`NewEnumerator2`
          (`self.Chase Player`))))))

(event `MoveToRandomLocation`
  (`|AIMoveTo` self (`NavigationSystemV1.K2_GetRandomReachablePointInRadius` (`self.K2_GetActorLocation`) 500.0 null null) null
    (:`then`
      (`KismetSystemLibrary.Delay` 1.0)
      (goto _label))))

(event `self.ReceiveBeginPlay`
  (switch `/Game/BluePrints/EAIState` (`self.AIState`)
    (:`NewEnumerator1`
      (`self.MoveToRandomLocation`))
    (:`NewEnumerator2`
      (`self.Chase Player`))))

(event `self.PawnSensing.OnSeePawn`
  (params (Pawn :type "Pawn Object Reference"))
  (cast `/Game/BluePrints/BP_Player` Pawn)
  (set `self.AIState` "NewEnumerator2")
  (`KismetSystemLibrary.RetriggerableDelay` 0.6)
  (set `self.AIState` "NewEnumerator1"))

(event `self.Sphere.OnComponentBeginOverlap`
  (params (OverlappedComponent :type "PrimitiveComponent Object Reference") (OtherActor :type "Actor Object Reference") (OtherComp :type "PrimitiveComponent Object Reference") (OtherBodyIndex :type Integer) (bFromSweep :type Boolean) (SweepResult :type "HitResult Structure (by ref)"))
  (cast `/Game/BluePrints/BP_Player` OtherActor)
  (`self.K2_DestroyActor`))

(fn `UserConstructionScript`)